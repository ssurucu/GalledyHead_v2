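; BP_FailteFactorGlobalManager is a manager actor that tracks the Failte Factor value and keeps the player's UI in sync with it.
; On BeginPlay it pushes a hardcoded starting value to the BP_FPS_Player UI without setting the stored value.
; ChangeFailteFactor applies a delta only if the result stays within the min and max limits, rejecting rather than clamping, then updates the UI and returns the new value.
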(event EventBeginPlay
  (bind _asbp_fps_player (Utilities|Casting|CastToBP_FPS_Player (Game|Player|GetPlayerPawn 0)))
  (Default|ChangeFailteFactorUIValue _asbp_fps_player 30))

(event Collision|EventActorBeginOverlap
  (params (OtherActor :type Actor%20Object%20Reference)))

(event EventTick
  (params (DeltaSeconds :type Float%20%28single-precision%29)))

(fn ConstructionScript)

(fn ChangeFailteFactor
  (params (Delta :type Integer))
  (Variables|Default|SetDelta Delta)
  (if (and (<= (+ (Variables|Default|GetFailteFactorValue) (Variables|Default|GetDelta)) (Variables|Default|GetMaxFailteFactorValue)) (>= (+ (Variables|Default|GetFailteFactorValue) (Variables|Default|GetDelta)) (Variables|Default|GetMinFailteFactorValue)))
    (bind _output_get (Variables|Default|SetFailteFactorValue (+ (Variables|Default|GetFailteFactorValue) (Variables|Default|GetDelta))))
    (bind _asbp_fps_player (Utilities|Casting|CastToBP_FPS_Player (Game|Player|GetPlayerPawn 0)))
    (Default|ChangeFailteFactorUIValue _asbp_fps_player _output_get)
    (return _output_get)))