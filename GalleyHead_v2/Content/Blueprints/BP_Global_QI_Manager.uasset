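; Global quest and inventory manager that links item changes to quest progress through event dispatchers.
; Inventory add and remove functions update an item-to-quantity map, save it, refresh the list widget and broadcast item updates.
; HandleItemUpdates completes quest objectives, and active quests broadcast their first unfinished objective on load, addition or item handling.
; The save load/create chain is disconnected; quest, dialogue and minigame handlers are stubs.
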(event Custom|QuestsLoad
  ;[0.15 0.15 0.15 0.5] BindLoadActiveQuests
  (CallFunction|QUEGetActiveQuests))

(event Custom|CustomEvent_2
  (params (QuestID :type Name) (QuestInfo :type ST%20Quest%20Info%20Structure) (MultipleQuestsAdded? :type Boolean))
  ;[0.15 0.15 0.15 0.5] BindLoadActiveQuests
  (CallFunction|QUEGetActiveQuests))

(event Custom|Event_DialogueUpdates
  ;[0.0405 0.15 0.1086 0.733] Event Listening
  (Development|PrintString "Event Dispatch: Dialogue Updates"))

(event Custom|Event_MiniGameUpdates
  ;[0.0405 0.15 0.1086 0.733] Event Listening
  (Development|PrintString "Event Dispatch: MiniGame Updates"))

(event EventBeginPlay
  (Utilities|FlowControl|Sequence
    (:then_0
      ;[0.08605 0.15 0.05613 0.5] Load the Inventory UI
      (bind _returnvalue (UserInterface|CreateWidget "/Game/UI/Inventory/BP_InventoryListView.BP_InventoryListView_C" (Game|GetPlayerController 0)))
      (bind _output_get (Variables|Default|SetInventoryListViewWidget _returnvalue))
      (UserInterface|Viewport|AddtoViewport _output_get 0))
    (:then_1
      (bind _asbp_fps_main (Utilities|Casting|CastToBP_FPS_Main (Game|GetPlayerCharacter 0)))
      (Variables|Default|SetPlayerQuestComponent (Variables|/Game/Blueprints/Mountea_Dialogue/BP_FPS_Main.BP_FPS_Main_C|GetBPC_PlayerQuestComponent _asbp_fps_main)))
    (:then_3
      ;[0.15 0.15 0.15 0.5] BindLoadActiveQuests
      (EventDispatchers|BindEventtoOnQuestsLoaded (Variables|Default|GetPlayerQuestComponent) (delegate Custom|QuestsLoad))
      (EventDispatchers|BindEventtoOnQuestAdded (Variables|Default|GetPlayerQuestComponent) (delegate Custom|CustomEvent_2)))
    (:then_4
      ;[0.0405 0.15 0.1086 0.733] Event Listening
      (EventDispatchers|BindEventtoOnItemUpdates (EventDispatchers|CreateEvent :!event HandleItemUpdates))
      ;;[0.15 0.15 0.15 0.5] Do we need this?
      (EventDispatchers|BindEventtoOnQuestUpdates (EventDispatchers|CreateEvent :!event HandleQuestUpdates))
      (EventDispatchers|BindEventtoOnDialogueUpdates (delegate Custom|Event_DialogueUpdates))
      (EventDispatchers|BindEventtoOnMiniGameUpdates (delegate Custom|Event_MiniGameUpdates)))))

(fn ConstructionScript)

(fn UpdateInventoryUI
  (params (PlayerInventoryList :type Map%20of%20BPS%20Inventory%20Item%20Structures%20to%20Integers))
  (LocalVariables|SetInventoryList PlayerInventoryList)
  (bind _asbp_inventory_list_view (Utilities|Casting|CastToBP_InventoryListView (Variables|Default|GetInventoryListViewWidget)))
  (Class|ListView|ClearListItems (Variables|/Game/UI/Inventory/BP_InventoryListView.BP_InventoryListView_C|Getinventory_list_view _asbp_inventory_list_view))
  (bind _keys (Utilities|Map|Keys (LocalVariables|GetInventoryList)))
  (for _array_element _keys
    (bind _returnvalue (Game|ConstructObjectfromClass "/Game/UI/Inventory/BP_InventoryListUIObject.BP_InventoryListUIObject_C" (Utilities|Struct|MakeBPS_InventoryItem (.ID (Utilities|Struct|BreakBPS_InventoryItem _array_element)) (.ReadableName (Utilities|Struct|BreakBPS_InventoryItem _array_element)) (.Value (Utilities|Map|Find (LocalVariables|GetInventoryList) _array_element)))))
    (Class|ListView|AddItem (Variables|/Game/UI/Inventory/BP_InventoryListView.BP_InventoryListView_C|Getinventory_list_view _asbp_inventory_list_view) _returnvalue)))

(fn SaveGameInventory
  (Variables|/Game/Blueprints/BP_SaveGame.BP_SaveGame_C|SetSavedInventory (Variables|Default|GetSavedGameState) (Variables|Default|GetPlayerInventory))
  (SaveGame|SaveGametoSlot (Variables|Default|GetSavedGameState) "LanternKeepSaveSlot"))

(fn INVAddItemtoInventory
  (params (Quantity :type Integer) (NewItem :type BP%20Quest%20Item%20Object%20Reference))
  (bind _itemuniquename (Variables|/Game/Blueprints/QuestItem_v2/BP_QuestItem.BP_QuestItem_C|GetItemUniqueName NewItem))
  (bind _returnvalue (Utilities|String|StringToName _itemuniquename))
  (LocalVariables|SetItemQuantity Quantity)
  (LocalVariables|SetNewItemQuestID (Variables|/Game/Blueprints/QuestItem_v2/BP_QuestItem.BP_QuestItem_C|GetQuestID NewItem))
  (LocalVariables|SetNewItemObjectiveID (Variables|/Game/Blueprints/QuestItem_v2/BP_QuestItem.BP_QuestItem_C|GetObjectiveID NewItem))
  (LocalVariables|SetItemToAdd (Utilities|Struct|MakeBPS_InventoryItem _returnvalue _returnvalue))
  (if (Utilities|Map|Contains (Variables|Default|GetPlayerInventory) (LocalVariables|GetItemToAdd))
    (if (.ReturnValue (Utilities|Map|Find (Variables|Default|GetPlayerInventory) (LocalVariables|GetItemToAdd)))
      (Utilities|Map|Add (Variables|Default|GetPlayerInventory) (LocalVariables|GetItemToAdd) (+ (.Value (Utilities|Map|Find (Variables|Default|GetPlayerInventory) (LocalVariables|GetItemToAdd))) (LocalVariables|GetItemQuantity)))
      (CallFunction|SaveGameInventory :!label _label)
      (CallFunction|UpdateInventoryUI (Variables|Default|GetPlayerInventory))
      (Default|CallOnItemUpdates (Utilities|Struct|MakeBPS_ItemUpdatePayload (.id (LocalVariables|GetItemToAdd)) false false) "NewEnumerator0" (LocalVariables|GetNewItemQuestID) (LocalVariables|GetNewItemObjectiveID)))
    (else
      (Utilities|Map|Add (Variables|Default|GetPlayerInventory) (LocalVariables|GetItemToAdd) (LocalVariables|GetItemQuantity))
      (bind _asbp_inventory_list_view (Utilities|Casting|CastToBP_InventoryListView (Variables|Default|GetInventoryListViewWidget)))
      (bind _returnvalue_2 (Game|ConstructObjectfromClass "/Game/UI/Inventory/BP_InventoryListUIObject.BP_InventoryListUIObject_C" (LocalVariables|GetItemToAdd)))
      (Class|ListView|AddItem (Variables|/Game/UI/Inventory/BP_InventoryListView.BP_InventoryListView_C|Getinventory_list_view _asbp_inventory_list_view) _returnvalue_2)
      (goto _label))))

(fn INVCheckifIteminInventory
  (params (ItemID :type Name))
  (return (Utilities|Map|Contains (Variables|Default|GetPlayerInventory) (Utilities|Struct|MakeBPS_InventoryItem ItemID ItemID))))

(fn INVRemoveAnItemfromInventory
  (params (QuantityToRemove :type Integer) (ItemToRemove :type BP%20Quest%20Item%20Object%20Reference) (RemovalMode :type ERemovalMode%20Enum :default "NewEnumerator0"))
  (bind _itemuniquename (Variables|/Game/Blueprints/QuestItem_v2/BP_QuestItem.BP_QuestItem_C|GetItemUniqueName ItemToRemove))
  (bind _returnvalue (Utilities|String|StringToName _itemuniquename))
  (LocalVariables|SetItemQuantityToRemove QuantityToRemove)
  (LocalVariables|SetItemToBeRemoved 0)
  (LocalVariables|SetItemIDToRemove (Utilities|Struct|MakeBPS_InventoryItem _returnvalue _returnvalue))
  (switch Utilities|FlowControl|Switch|SwitchonERemovalMode RemovalMode
    (:NewEnumerator0
      (Utilities|Map|Add (Variables|Default|GetPlayerInventory) (LocalVariables|GetItemIDToRemove) (- (.Value (Utilities|Map|Find (Variables|Default|GetPlayerInventory) (LocalVariables|GetItemIDToRemove))) 1)))
    (:NewEnumerator1
      (Utilities|Map|Add (Variables|Default|GetPlayerInventory) (LocalVariables|GetItemIDToRemove) (- (.Value (Utilities|Map|Find (Variables|Default|GetPlayerInventory) (LocalVariables|GetItemIDToRemove))) (LocalVariables|GetItemQuantityToRemove))))
    (:NewEnumerator2
      (Utilities|Map|Remove (Variables|Default|GetPlayerInventory) (LocalVariables|GetItemIDToRemove))))
  (Development|PrintString "Dlete successfully")
  (CallFunction|SaveGameInventory)
  (CallFunction|UpdateInventoryUI (Variables|Default|GetPlayerInventory))
  (Default|CallOnItemUpdates (Utilities|Struct|MakeBPS_ItemUpdatePayload (.id (LocalVariables|GetItemIDToRemove)) false false) "NewEnumerator1" (Variables|/Game/Blueprints/QuestItem_v2/BP_QuestItem.BP_QuestItem_C|GetQuestID (LocalVariables|GetItemToBeRemoved)) (Variables|/Game/Blueprints/QuestItem_v2/BP_QuestItem.BP_QuestItem_C|GetObjectiveID (LocalVariables|GetItemToBeRemoved))))

(fn INVInitializeInventory
  (bind _output_get (Variables|Default|SetPlayerInventory (Variables|/Game/Blueprints/BP_SaveGame.BP_SaveGame_C|GetSavedInventory (Variables|Default|GetSavedGameState))))
  (if (> (Utilities|Map|Length _output_get) 0)
    _
    (else
      (Development|PrintString "No items in the inventory")))
  (CallFunction|SaveGameInventory)
  (CallFunction|UpdateInventoryUI (Variables|Default|GetPlayerInventory)))

(fn HandleItemUpdates
  (params (ItemUpdatePayload :type BPS%20Item%20Update%20Payload%20Structure) (Action :type EInventoryItemUpdates%20Enum :default "NewEnumerator0") (QuestID :type Name) (ObjectiveID :type Name))
  (Development|PrintString "Event Dispatch: Item Updates")
  (switch Utilities|FlowControl|Switch|SwitchonEInventoryItemUpdates "NewEnumerator0"
    (:NewEnumerator0
      (Default|CompleteObjective (Variables|Default|GetBP_QuestHandlerComponent) QuestID ObjectiveID)
      (CallFunction|QUEGetActiveQuests))))

(fn HandleQuestUpdates
  (params (UpdateType :type EQuestUpdates%20Enum :default "NewEnumerator0") (QuestID :type Name) (ObjetiveID :type Name))
  (LocalVariables|SetL_QuestID QuestID)
  (LocalVariables|SetL_ObjectiveID ObjetiveID)
  (switch Utilities|FlowControl|Switch|SwitchonEQuestUpdates UpdateType))

(fn QUEGetActiveQuests
  (for _array_element (Variables|/Game/Blueprints/Add-ons/EasyQuests/Blueprints/BP_BPC_PlayerQuestComponent.BP_BPC_PlayerQuestComponent_C|GetActiveQuests (Variables|Default|GetPlayerQuestComponent))
    (bind _array_element_2 (Utilities|Array|ForEachLoopwithBreak (.objectives _array_element) :!label _label)
      (:LoopBody
        (if (< (.currentamount _array_element_2) (.requiredamount _array_element_2))
          (Default|CallOnQuestUpdates "NewEnumerator3" (.questid _array_element) (.objective_id _array_element_2))
          (goto _label Break))))))