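; Quest handler component that relays player quest events to its owning BP_Global_QI_Manager.
; On BeginPlay it binds to the FPS player's quest component delegates for quest added, completed and objective updated.
; Start and complete broadcast OnQuestUpdates without IDs, and start also passes accumulated quests to the active NPC's ImitiateOnInteract.
; CompleteObjective increments objective progress and broadcasts, but the objective-updated handler is an untested, empty stub.
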(event Custom|Event_StartQuest
  (params (QuestID :type Name) (QuestInfo :type ST%20Quest%20Info%20Structure) (MultipleQuestsAdded? :type Boolean))
  (CallFunction|StartQuest QuestID))

(event Custom|Event_CompleteQuest
  (params (QuestID :type Name) (Quest :type ST%20Quest%20Info%20Structure))
  (CallFunction|CompleteQuest QuestID))

(event Custom|Event_ObjUpdated
  (params (ObjectiveID :type Name) (Objective :type ST%20Quest%20Objectives%20Structure) (QuestInfo :type ST%20Quest%20Info%20Structure))
  ;[0.15 0.15 0.15 0.5] Objective Update has to be tested, not sure if we're getting this when an objective is completed
)

(event EventBeginPlay
  (bind _asbp_fps_main (Utilities|Casting|CastToBP_FPS_Main (Game|Player|GetPlayerPawn 0)))
  (EventDispatchers|BindEventtoOnQuestAdded (Variables|/Game/Blueprints/Mountea_Dialogue/BP_FPS_Main.BP_FPS_Main_C|GetBPC_PlayerQuestComponent _asbp_fps_main) (delegate Custom|Event_StartQuest))
  (EventDispatchers|BindEventtoOnQuestCompleted (Variables|/Game/Blueprints/Mountea_Dialogue/BP_FPS_Main.BP_FPS_Main_C|GetBPC_PlayerQuestComponent _asbp_fps_main) (delegate Custom|Event_CompleteQuest))
  ;[0.15 0.15 0.15 0.5] Objective Update has to be tested, not sure if we're getting this when an objective is completed
  (EventDispatchers|BindEventtoOnObjectiveUpdated (Variables|/Game/Blueprints/Mountea_Dialogue/BP_FPS_Main.BP_FPS_Main_C|GetBPC_PlayerQuestComponent _asbp_fps_main) (delegate Custom|Event_ObjUpdated)))

(fn CompleteQuest
  (params (QuestID :type Name))
  (bind _asbp_global_qi_manager (Utilities|Casting|CastToBP_Global_QI_Manager (Components|GetOwner)))
  (Default|CallOnQuestUpdates _asbp_global_qi_manager "NewEnumerator0")
  (return true))

(fn CompleteObjective
  (params (QuestID :type Name) (ObjectiveID :type Name))
  (bind _asbp_fps_main (Utilities|Casting|CastToBP_FPS_Main (Game|GetPlayerCharacter 0)))
  (Default|AddObjectiveAmount (Variables|/Game/Blueprints/Mountea_Dialogue/BP_FPS_Main.BP_FPS_Main_C|GetBPC_PlayerQuestComponent _asbp_fps_main) QuestID ObjectiveID 1)
  (bind _asbp_global_qi_manager (Utilities|Casting|CastToBP_Global_QI_Manager (Components|GetOwner)))
  (Default|CallOnQuestUpdates _asbp_global_qi_manager "NewEnumerator2")
  (return true))

(fn StartQuest
  (params (QuestID :type Name))
  (bind _asbp_global_qi_manager (Utilities|Casting|CastToBP_Global_QI_Manager (Components|GetOwner)))
  (Utilities|Array|Add (LocalVariables|GetQuestsToAssign) QuestID)
  (Default|ImitiateonInteract (Variables|/Game/Blueprints/BP_Global_QI_Manager.BP_Global_QI_Manager_C|GetActiveNPC _asbp_global_qi_manager) (LocalVariables|GetQuestsToAssign))
  (bind _asbp_global_qi_manager_2 (Utilities|Casting|CastToBP_Global_QI_Manager (Components|GetOwner)))
  (Default|CallOnQuestUpdates _asbp_global_qi_manager_2 "NewEnumerator1")
  (return true))